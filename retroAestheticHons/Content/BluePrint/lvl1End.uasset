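; Level 1 end actor that stays hidden until the player has made enough BR74 kills.
; On BeginPlay it hides itself and turns off its Box collision.
; Every Tick it casts the player character to Z15 and checks BR74KillCount, revealing itself and enabling query-only collision once the count reaches five.
; The file contains no active overlap logic, so this Blueprint only handles the unlock.
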(event `self.ReceiveBeginPlay`
  (`self.SetActorHiddenInGame` true)
  (`PrimitiveComponent.SetCollisionEnabled` (`self.Box`) "NoCollision"))

(event `Br74Killcheck`
  (bind _asz15 (cast `/Game/BluePrint/Z15` (`GameplayStatics.GetPlayerCharacter` 0)))
  (if (>= (`/Game/BluePrint/Z15.BR74KillCount` _asz15) 5)
    (`PrimitiveComponent.SetCollisionEnabled` (`self.Box`) "QueryOnly")
    (`self.SetActorHiddenInGame` false)))

(event `self.ReceiveTick`
  (params (DeltaSeconds :type "Float (single-precision)"))
  (`self.Br74Killcheck`))

(fn `UserConstructionScript`)