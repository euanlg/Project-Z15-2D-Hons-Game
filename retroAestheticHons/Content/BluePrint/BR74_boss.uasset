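; BR74 boss: a sprite-based enemy that yaws to face the player and escalates its attack as health drops.
; Tick drives three health phases: one sweeping bullet arrow, then a second, then periodic BR74 minion spawns in Box11.
; Arrow pitch steps each shot cycle, reversing at exactly 90; the -90 reversal events are never called.
; DoOnce-plus-Delay gates throttle firing, spawning and damage intake, and the boss is destroyed at zero health.
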(event `Shoot2`
  (bind (_returnvalue_location _returnvalue_rotation) (`KismetMathLibrary.BreakTransform` (`SceneComponent.K2_GetComponentToWorld` (`self.Arrow1`))))
  (`/Engine/EditorBlueprintResources/StandardMacros.DoOnce` false :!label _label
    (:`Completed`
      (`|SpawnActorFromClass` "/Game/BluePrint/BR74BossBullet.BR74BossBullet_C" (`KismetMathLibrary.MakeTransform` _returnvalue_location _returnvalue_rotation) "Undefined" "OverrideRootScale" null null)
      (`GameplayStatics.PlaySoundAtLocation` "/Game/Audio/lazer2_Cue.lazer2_Cue")
      (`KismetSystemLibrary.Delay` 0.3)
      (goto _label :!via `Reset`))))

(event `ArchShoot2`
  ;[1 1 1] Arch Shoot 2
  (`KismetSystemLibrary.Delay` 0.0005)
  (if (`KismetMathLibrary.InRange_FloatFloat` (`self.RotY_0`) -180.0 90.0)
    (`self.Shoot2`)
    (`SceneComponent.K2_SetWorldRotation` (`self.Arrow1`) (`KismetMathLibrary.MakeRotator` (`self.RotX_0`) (+ (`self.RotY_0`) (`self.YMovementShoot_0`)) (`self.RotZ_0`)) false false)
    (`self.Get Other Arrow Rot`)))

(event `self.ReceiveBeginPlay`
  (set `self.RotY` -180.0)
  (set `self.RotY_0` -180.0)
  (set `self.YMovementShoot` 1.0)
  (set `self.YMovementShoot_0` 2.0))

(event `ArchShoot`
  ;[1 1 1] Arch Shoot
  (`KismetSystemLibrary.Delay` 0.0005)
  (if (`KismetMathLibrary.InRange_FloatFloat` (`self.RotY`) -180.0 90.0)
    (`self.BR74_Shoot`)
    (`SceneComponent.K2_SetWorldRotation` (`self.Arrow`) (`KismetMathLibrary.MakeRotator` (`self.RotX`) (+ (`self.RotY`) (`self.YMovementShoot`)) (`self.RotZ`)) false false)
    (`self.Get arrow rotation`)))

(event `Ifshootangle90`
  ;[1 1 1] Invertshooit angle
  (if (== (`self.RotY`) 90.0)
    (set `self.YMovementShoot` -1.0)))

(event `2nDshootAngle90`
  ;[1 1 1] Other Shoot Angle Invert
  (if (== (`self.RotY_0`) 90.0)
    (set `self.YMovementShoot_0` -1.0)))

(event `ifshootangle-90`
  ;[1 1 1] Invertshooit angle
  (if (== (`self.RotY`) -90.0)
    (set `self.YMovementShoot` 1.0)))

(event `2nDShootAngle-90`
  ;[1 1 1] Other Shoot Angle Invert
  (if (== (`self.RotY_0`) -90.0)
    (set `self.YMovementShoot_0` 1.0)))

(event `Get arrow rotation`
  (bind (_relativerotation_roll _relativerotation_pitch _relativerotation_yaw) (`KismetMathLibrary.BreakRotator` (`SceneComponent.RelativeRotation` (`self.Arrow`))))
  ;[1 1 1] Get arrow rotation
  (`|ExecutionSequence`
    (:`then_0`
      (set `self.RotX` _relativerotation_roll))
    (:`then_1`
      (set `self.RotY` _relativerotation_pitch))
    (:`then_2`
      (set `self.RotZ` _relativerotation_yaw))))

(event `Get Other Arrow Rot`
  (bind (_relativerotation_roll _relativerotation_pitch _relativerotation_yaw) (`KismetMathLibrary.BreakRotator` (`SceneComponent.RelativeRotation` (`self.Arrow1`))))
  ;[1 1 1] Get other arrow rotation
  (`|ExecutionSequence`
    (:`then_0`
      (set `self.RotX_0` _relativerotation_roll))
    (:`then_1`
      (set `self.RotY_0` _relativerotation_pitch))
    (:`then_2`
      (set `self.RotZ_0` _relativerotation_yaw))))

(event `DMG_BR74`
  (params (NewParamDMGTaken :type Integer))
  ;[1 1 1] Take Damage
  (`/Engine/EditorBlueprintResources/StandardMacros.DoOnce` false :!label _label_2
    (:`Completed`
      (bind _output_get (set `self.BR74Health` (- (`self.BR74Health`) NewParamDMGTaken)))
      (if (<= _output_get 0)
        (`KismetSystemLibrary.Delay` 0.2)
        (`self.K2_DestroyActor`)
        (else
          (`KismetSystemLibrary.PrintString` (`KismetStringLibrary.Conv_IntToString` (`self.BR74Health`)))
          (`KismetSystemLibrary.Delay` 0.2)
          (goto _label_2 :!via `Reset`))))))

(event `GetPlayerDistance`
  (bind _returnvalue_x (`KismetMathLibrary.BreakVector` (`self.K2_GetActorLocation` (`GameplayStatics.GetPlayerCharacter` 0))))
  (bind _returnvalue_x_2 (`KismetMathLibrary.BreakVector` (`SceneComponent.K2_GetComponentLocation` (`self.PaperSprite`))))
  (bind (_returnvalue_x_3 _returnvalue_y _returnvalue_z) (`KismetMathLibrary.BreakVector` (`self.K2_GetActorLocation` (`GameplayStatics.GetPlayerCharacter` 0))))
  (bind (_returnvalue_x_4 _returnvalue_y_2 _returnvalue_z_2) (`KismetMathLibrary.BreakVector` (`SceneComponent.K2_GetComponentLocation` (`self.PaperSprite`))))
  ;[1 1 1] get player distance
  (`|ExecutionSequence`
    (:`then_0`
      (set `self.DistanceX` (- _returnvalue_x_2 _returnvalue_x)))
    (:`then_1`
      (set `self.DistanceZ` (- _returnvalue_z_2 _returnvalue_z)))))

(event `Get PLayer Location`
  (bind (_returnvalue_x _returnvalue_y _returnvalue_z) (`KismetMathLibrary.BreakVector` (`self.K2_GetActorLocation`)))
  ;[1 1 1] Get player Location
  (`|ExecutionSequence`
    (:`then_0`
      (set `self.ActorX` _returnvalue_x))
    (:`then_1`
      (set `self.ActorY` _returnvalue_y))
    (:`then_2`
      (set `self.ActorZ` _returnvalue_z))))

(event `BR74_Shoot`
  (bind (_returnvalue_location _returnvalue_rotation) (`KismetMathLibrary.BreakTransform` (`SceneComponent.K2_GetComponentToWorld` (`self.Arrow`))))
  ;[1 1 1] Shoot
  (`/Engine/EditorBlueprintResources/StandardMacros.DoOnce` false :!label _label_3
    (:`Completed`
      (`|SpawnActorFromClass` "/Game/BluePrint/BR74BossBullet.BR74BossBullet_C" (`KismetMathLibrary.MakeTransform` _returnvalue_location _returnvalue_rotation) "Undefined" "OverrideRootScale" null null)
      (`GameplayStatics.PlaySoundAtLocation` "/Game/Audio/lazer2_Cue.lazer2_Cue")
      (`KismetSystemLibrary.Delay` 0.2)
      (goto _label_3 :!via `Reset`))))

(event `SpawnBR74`
  (bind _box11 (`self.Box11`))
  ;[1 1 1] Spawn Small Br74
  (`/Engine/EditorBlueprintResources/StandardMacros.DoOnce` false :!label _label_4
    (:`Completed`
      (`|SpawnActorFromClass` "/Game/BluePrint/BR74.BR74_C" (`KismetMathLibrary.Conv_VectorToTransform` (`KismetMathLibrary.RandomPointInBoundingBox` (`SceneComponent.RelativeLocation` _box11) (`BoxComponent.BoxExtent` _box11))) "AlwaysSpawn" "OverrideRootScale" null null)
      (`KismetSystemLibrary.Delay` 5.0)
      (goto _label_4 :!via `Reset`))))

(event `Look at player X`
  (bind (_returnvalue_roll _returnvalue_pitch _returnvalue_yaw) (`KismetMathLibrary.BreakRotator` (`KismetMathLibrary.FindLookAtRotation` (`self.K2_GetActorLocation`) (`self.K2_GetActorLocation` (`GameplayStatics.GetPlayerCharacter` 0)))))
  ;[1 1 1] look at player x
  (`self.K2_SetActorRotation` (`KismetMathLibrary.MakeRotator` 0.0 0.0 _returnvalue_yaw)))

(event `self.ReceiveTick`
  (params (DeltaSeconds :type "Float (single-precision)"))
  (bind _br74health (`self.BR74Health`))
  (bind _br74health_2 (`self.BR74Health`))
  (bind _br74health_3 (`self.BR74Health`))
  (`|ExecutionSequence`
    (:`then_0`
      (`self.Get PLayer Location`)
      (`self.GetPlayerDistance`)
      (`self.Look at player X`))
    (:`then_1`
      (if (and (<= _br74health_2 300) (>= _br74health_2 200))
        (`self.ifshootangle-90`)
        (`self.Ifshootangle90`)
        (`self.ArchShoot`)))
    (:`then_2`
      (if (and (<= _br74health_3 200) (>= _br74health_3 100))
        (`|ExecutionSequence`
          (:`then_0`
            (`self.ifshootangle-90`)
            (`self.Ifshootangle90`)
            (`self.ArchShoot`))
          (:`then_1`
            (`self.2nDShootAngle-90`)
            (`self.2nDshootAngle90`)
            (`self.ArchShoot2`)))))
    (:`then_3`
      (if (and (<= _br74health 100) (>= _br74health 1))
        (`|ExecutionSequence`
          (:`then_0`
            (`self.ifshootangle-90`)
            (`self.Ifshootangle90`)
            (`self.ArchShoot`))
          (:`then_1`
            (`self.2nDShootAngle-90`)
            (`self.2nDshootAngle90`)
            (`self.ArchShoot2`))
          (:`then_2`
            (`self.SpawnBR74`)))))))

(fn `UserConstructionScript`)