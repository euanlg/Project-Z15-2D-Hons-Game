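; BR74 is a Paper2D enemy actor that tracks, approaches and shoots at the player on the X/Z plane.
; Tick yaws it toward the player and uses signed X/Z offsets to trigger firing and delayed one-unit steps that close in or back off.
; DoOnce-plus-Delay gates throttle bullet spawning and incoming damage.
; At zero health it destroys itself and calls EnergyZ15 on the Z15 player.
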(event `DMG_BR74`
  (params (NewParamDMGTaken :type Integer))
  (`/Engine/EditorBlueprintResources/StandardMacros.DoOnce` false :!label _label
    (:`Completed`
      (bind _output_get (set `self.BR74Health` (- (`self.BR74Health`) NewParamDMGTaken)))
      (if (<= _output_get 0)
        (`KismetSystemLibrary.Delay` 0.2)
        (`self.K2_DestroyActor`)
        (bind _asz15 (cast `/Game/BluePrint/Z15` (`GameplayStatics.GetPlayerCharacter` 0)))
        (`/Game/BluePrint/Z15.energy_z15` _asz15 10)
        (else
          (`KismetSystemLibrary.PrintString` (`KismetStringLibrary.Conv_IntToString` (`self.BR74Health`)))
          (`KismetSystemLibrary.Delay` 0.2)
          (goto _label :!via `Reset`))))))

(event `BR74_Shoot`
  (`/Engine/EditorBlueprintResources/StandardMacros.DoOnce` false :!label _label_2
    (:`Completed`
      (`|SpawnActorFromClass` "/Game/BluePrint/BR74_Bullet.BR74_Bullet_C" (`SceneComponent.K2_GetComponentToWorld` (`self.Arrow`)) "Undefined" "OverrideRootScale" null null)
      (`GameplayStatics.PlaySoundAtLocation` "/Game/Audio/lazer2.lazer2")
      (`KismetSystemLibrary.Delay` 1.3)
      (goto _label_2 :!via `Reset`))))

(event `self.ReceiveTick`
  (params (DeltaSeconds :type "Float (single-precision)"))
  (bind (_returnvalue_x _returnvalue_y _returnvalue_z) (`KismetMathLibrary.BreakVector` (`self.K2_GetActorLocation`)))
  (bind _returnvalue_x_2 (`KismetMathLibrary.BreakVector` (`self.K2_GetActorLocation` (`GameplayStatics.GetPlayerCharacter` 0))))
  (bind _returnvalue_x_3 (`KismetMathLibrary.BreakVector` (`SceneComponent.K2_GetComponentLocation` (`self.PaperSprite`))))
  (bind (_returnvalue_x_4 _returnvalue_y_2 _returnvalue_z_2) (`KismetMathLibrary.BreakVector` (`self.K2_GetActorLocation` (`GameplayStatics.GetPlayerCharacter` 0))))
  (bind (_returnvalue_x_5 _returnvalue_y_3 _returnvalue_z_3) (`KismetMathLibrary.BreakVector` (`SceneComponent.K2_GetComponentLocation` (`self.PaperSprite`))))
  (bind (_returnvalue_roll _returnvalue_pitch _returnvalue_yaw) (`KismetMathLibrary.BreakRotator` (`KismetMathLibrary.FindLookAtRotation` (`self.K2_GetActorLocation`) (`self.K2_GetActorLocation` (`GameplayStatics.GetPlayerCharacter` 0)))))
  (`|ExecutionSequence`
    (:`then_0`
      (`|ExecutionSequence`
        (:`then_0`
          (bind _output_get (set `self.DistanceX` (- _returnvalue_x_3 _returnvalue_x_2))))
        (:`then_1`
          (bind _output_get_2 (set `self.DistanceZ` (- _returnvalue_z_3 _returnvalue_z_2)))
          (if (and (<= _output_get 100.0) (<= _output_get_2 25.0))
            (`self.BR74_Shoot`)))))
    (:`then_1`
      (`self.K2_SetActorRotation` (`KismetMathLibrary.MakeRotator` 0.0 0.0 _returnvalue_yaw)))
    (:`then_2`
      (set `self.ActorX` _returnvalue_x))
    (:`then_3`
      (set `self.ActorY` _returnvalue_y))
    (:`then_4`
      (set `self.ActorZ` _returnvalue_z))
    (:`then_5`
      (if (not (or (>= (`self.DistanceX`) 180.0) (>= (`self.DistanceZ`) 180.0)))
        (`self.move to player`)))))

(event `move to player`
  ;[1 1 1] move to player
  (`|ExecutionSequence`
    (:`then_0`
      (if (`KismetMathLibrary.InRange_FloatFloat` (`self.DistanceX`) 20.0 150.0)
        (`KismetSystemLibrary.Delay` 0.04)
        (`self.K2_SetActorLocation` (`KismetMathLibrary.MakeVector` (+ (`self.ActorX`) -1.0) (`self.ActorY`) (`self.ActorZ`)))
        (elif (`KismetMathLibrary.InRange_FloatFloat` (`self.DistanceX`) -150.0 -20.0)
          (`KismetSystemLibrary.Delay` 0.04)
          (`self.K2_SetActorLocation` (`KismetMathLibrary.MakeVector` (+ (`self.ActorX`) 1.0) (`self.ActorY`) (`self.ActorZ`))))))
    (:`then_1`
      (if (`KismetMathLibrary.InRange_FloatFloat` (`self.DistanceZ`) 10.0 150.0)
        (`KismetSystemLibrary.Delay` 0.04)
        (`self.K2_SetActorLocation` (`KismetMathLibrary.MakeVector` (`self.ActorX`) (`self.ActorY`) (+ (`self.ActorZ`) -1.0)))
        (elif (`KismetMathLibrary.InRange_FloatFloat` (`self.DistanceZ`) -150.0 -10.0)
          (`KismetSystemLibrary.Delay` 0.04)
          (`self.K2_SetActorLocation` (`KismetMathLibrary.MakeVector` (`self.ActorX`) (`self.ActorY`) (+ (`self.ActorZ`) 1.0))))))
    (:`then_2`
      (if (`KismetMathLibrary.InRange_FloatFloat` (`self.DistanceX`) 0.0 30.0)
        (`KismetSystemLibrary.Delay` 0.04)
        (`self.K2_SetActorLocation` (`KismetMathLibrary.MakeVector` (+ (`self.ActorX`) 1.0) (`self.ActorY`) (`self.ActorZ`)))
        (elif (`KismetMathLibrary.InRange_FloatFloat` (`self.DistanceX`) -30.0 0.0)
          (`KismetSystemLibrary.Delay` 0.04)
          (`self.K2_SetActorLocation` (`KismetMathLibrary.MakeVector` (+ (`self.ActorX`) -1.0) (`self.ActorY`) (`self.ActorZ`))))))
    (:`then_3`
      (if (`KismetMathLibrary.InRange_FloatFloat` (`self.DistanceZ`) 0.0 15.0)
        (`KismetSystemLibrary.Delay` 0.04)
        (`self.K2_SetActorLocation` (`KismetMathLibrary.MakeVector` (`self.ActorX`) (`self.ActorY`) (+ (`self.ActorZ`) 1.0)))
        (elif (`KismetMathLibrary.InRange_FloatFloat` (`self.DistanceZ`) -15.0 0.0)
          (`KismetSystemLibrary.Delay` 0.04)
          (`self.K2_SetActorLocation` (`KismetMathLibrary.MakeVector` (`self.ActorX`) (`self.ActorY`) (+ (`self.ActorZ`) -1.0))))))))

(fn `UserConstructionScript`)