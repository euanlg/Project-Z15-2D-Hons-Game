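; Spawner actor that releases a one-time batch of BR74 actors when a Z15 enters its trigger box.
; The box overlap casts to Z15 and passes through a DoOnce to spawnBr74.
; That event loops to spawn each BR74 at a random point within the box extent, ignoring collisions.
; The random points center on the box's relative location, used directly as world coordinates.
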(event `spawn Br74`
  (bind _box (`self.Box`))
  (for _ (range 6)
    (`|SpawnActorFromClass` "/Game/BluePrint/BR74.BR74_C" (`KismetMathLibrary.Conv_VectorToTransform` (`KismetMathLibrary.RandomPointInBoundingBox` (`SceneComponent.RelativeLocation` _box) (`BoxComponent.BoxExtent` _box))) "AlwaysSpawn" "OverrideRootScale" null null)))

(event `self.ReceiveTick`
  (params (DeltaSeconds :type "Float (single-precision)")))

(event `self.Box.OnComponentBeginOverlap`
  (params (OverlappedComponent :type "PrimitiveComponent Object Reference") (OtherActor :type "Actor Object Reference") (OtherComp :type "PrimitiveComponent Object Reference") (OtherBodyIndex :type Integer) (bFromSweep :type Boolean) (SweepResult :type "HitResult Structure (by ref)"))
  (cast `/Game/BluePrint/Z15` OtherActor)
  (`/Engine/EditorBlueprintResources/StandardMacros.DoOnce` false
    (:`Completed`
      (`self.spawn Br74`))))

(fn `UserConstructionScript`)