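; Projectile actor for a Paper2D game that damages BR74 actors on overlap and self-destructs after a short lifetime.
; Every tick nudges the flipbook's world Y slightly to either side of zero based on its yaw.
; A BR74 hit stops the projectile movement, applies fixed damage, disables collision, plays a sound at the world origin, and switches the flipbook from Idle to Boom before destroying the actor.
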(event `self.ReceiveBeginPlay`
  (`KismetSystemLibrary.Delay` 1.5)
  (`self.K2_DestroyActor`))

(event `YForward`
  (bind (_returnvalue_x _returnvalue_y _returnvalue_z) (`KismetMathLibrary.BreakVector` (`SceneComponent.K2_GetComponentLocation` (`self.PaperFlipbook`))))
  (bind (_returnvalue_roll _returnvalue_pitch _returnvalue_yaw) (`KismetMathLibrary.BreakRotator` (`SceneComponent.K2_GetComponentRotation` (`self.PaperFlipbook`))))
  (bind (_returnvalue_x_2 _returnvalue_y_2 _returnvalue_z_2) (`KismetMathLibrary.BreakVector` (`SceneComponent.K2_GetComponentLocation` (`self.PaperFlipbook`))))
  (if (== _returnvalue_yaw 180.0)
    (`SceneComponent.K2_SetWorldLocation` (`self.PaperFlipbook`) (`KismetMathLibrary.MakeVector` _returnvalue_x -0.1 _returnvalue_z) false false)
    (else
      (`SceneComponent.K2_SetWorldLocation` (`self.PaperFlipbook`) (`KismetMathLibrary.MakeVector` _returnvalue_x_2 0.1 _returnvalue_z_2) false false))))

(event `self.ReceiveTick`
  (params (DeltaSeconds :type "Float (single-precision)"))
  (`self.YForward`))

(event `self.Box.OnComponentBeginOverlap`
  (params (OverlappedComponent :type "PrimitiveComponent Object Reference") (OtherActor :type "Actor Object Reference") (OtherComp :type "PrimitiveComponent Object Reference") (OtherBodyIndex :type Integer) (bFromSweep :type Boolean) (SweepResult :type "HitResult Structure (by ref)"))
  (`self.YForward`)
  (bind _asbr74 (cast `/Game/BluePrint/BR74` OtherActor))
  (`|ExecutionSequence`
    (:`then_0`
      (`MovementComponent.StopMovementImmediately` (`self.ProjectileMovement`)))
    (:`then_1`
      (`/Game/BluePrint/BR74.DMG_BR74` _asbr74 34)
      (`PrimitiveComponent.SetCollisionEnabled` (`self.Box`) "NoCollision")
      (`self.State Switch` "NewEnumerator0")
      (`KismetSystemLibrary.Delay` 0.3)
      (`self.K2_DestroyActor`))
    (:`then_2`
      (`GameplayStatics.PlaySoundAtLocation` "/Game/Audio/boom_Cue.boom_Cue"))))

(fn `state switch`
  (params (Nextstate :type "/Game/BluePrint/bulletstate Enum" :default "NewEnumerator0"))
  (set `self.currentstate` Nextstate)
  (`PaperFlipbookComponent.SetFlipbook` (`self.PaperFlipbook`) (select `/Game/BluePrint/bulletstate` (`self.currentstate`) :`NewEnumerator0` (`self.boom`) :`NewEnumerator1` (`self.Idle`)))
  (return))

(fn `UserConstructionScript`)