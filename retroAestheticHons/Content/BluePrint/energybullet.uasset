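; Energy bullet actor that plays a timed charge, fire and fade sequence, then destroys itself.
; BeginPlay steps a state through Build, Full and End with delays, and StateSwitch swaps the Paper2D flipbook for each, with build and fire sounds.
; Box overlap waits briefly, then damages BR74 actors and plays a boom sound, in any state.
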(event `self.ReceiveBeginPlay`
  (`GameplayStatics.PlaySoundAtLocation` "/Game/Audio/build_Cue.build_Cue" (0.0 0.0 0.0) (struct) 0.5)
  (`self.StateSwitch` "NewEnumerator1")
  (`KismetSystemLibrary.Delay` 0.6)
  (`self.StateSwitch` "NewEnumerator0")
  (`GameplayStatics.PlaySoundAtLocation` "/Game/Audio/fire_Cue.fire_Cue")
  (`KismetSystemLibrary.Delay` 0.5)
  (`self.StateSwitch` "NewEnumerator2")
  (`KismetSystemLibrary.Delay` 0.4)
  (`self.K2_DestroyActor`))

(event `self.Box.OnComponentBeginOverlap`
  (params (OverlappedComponent :type "PrimitiveComponent Object Reference") (OtherActor :type "Actor Object Reference") (OtherComp :type "PrimitiveComponent Object Reference") (OtherBodyIndex :type Integer) (bFromSweep :type Boolean) (SweepResult :type "HitResult Structure (by ref)"))
  (`KismetSystemLibrary.Delay` 0.1)
  (bind _asbr74 (cast `/Game/BluePrint/BR74` OtherActor))
  (`/Game/BluePrint/BR74.DMG_BR74` _asbr74 51)
  (`GameplayStatics.PlaySoundAtLocation` "/Game/Audio/boom_Cue.boom_Cue"))

(fn `StateSwitch`
  (params (NextState :type "/Game/BluePrint/energystate Enum" :default "NewEnumerator0"))
  (set `self.CurrentState` NextState)
  (`PaperFlipbookComponent.SetFlipbook` (`self.PaperFlipbook`) (select `/Game/BluePrint/energystate` (`self.CurrentState`) :`NewEnumerator0` (`self.full`) :`NewEnumerator1` (`self.build`) :`NewEnumerator2` (`self.end`)))
  (return))

(fn `UserConstructionScript`)