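; Z15 is the player's side-scrolling flipbook character, with movement, jumping, gated auto-fire, and an energy-costed shield and charged shot.
; Tick updates facing, Idle/Run flipbooks, shot offsets and normalized health and energy floats.
; BeginPlay restores stats from the game instance, adds the HUD and places Z15 at the level's spawn.
; Kill-gated end overlaps advance the level by teleporting; death writes reset stats to the instance and reopens the map.
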(event `energy_z15`
  (params (EnergyAdded :type Integer))
  ;[1 1 1] add energy
  (bind _output_get (set `self.Energy` (+ (`self.Energy`) EnergyAdded)))
  (if (>= _output_get 100)
    (set `self.Energy` 100)
    (else
      (`KismetSystemLibrary.PrintString` (`KismetStringLibrary.Conv_IntToString` (`self.Energy`))))))

(event `self.ReceiveBeginPlay`
  ;[1 1 1] event beginplay
  (`|ExecutionSequence`
    (:`then_0`
      (bind _asgame_instance (cast `/Game/BluePrint/gameInstance` (`GameplayStatics.GetGameInstance`)))
      (`|ExecutionSequence`
        (:`then_0`
          (set `self.Energy` (`/Game/BluePrint/gameInstance.InsEnergy` _asgame_instance)))
        (:`then_1`
          (set `self.Z15_Health` (`/Game/BluePrint/gameInstance.InsHealth` _asgame_instance)))
        (:`then_2`
          (set `self.lvlcounter` (`/Game/BluePrint/gameInstance.InsLevel` _asgame_instance)))
        (:`then_3`
          (set `self.Spawn Loc` (`/Game/BluePrint/gameInstance.InsLoc` _asgame_instance)))))
    (:`then_1`
      (bind _returnvalue (`|CreateWidget` "/Game/BluePrint/hud.hud_C"))
      (`UserWidget.AddToViewport` _returnvalue 0))
    (:`then_2`
      (`self.Set Spawn`)
      (`SceneComponent.K2_SetWorldLocation` (`self.CapsuleComponent`) (`self.Spawn Loc`) false false))))

(event `IfDestroyed`
  ;[1 1 1] If Destroyed
  (bind _asgame_instance (cast `/Game/BluePrint/gameInstance` (`GameplayStatics.GetGameInstance`)))
  (`|ExecutionSequence`
    (:`then_0`
      (set `/Game/BluePrint/gameInstance.InsHealth` 100 _asgame_instance))
    (:`then_1`
      (set `/Game/BluePrint/gameInstance.InsEnergy` 50 _asgame_instance))
    (:`then_2`
      (set `/Game/BluePrint/gameInstance.InsLevel` (`self.lvlcounter`) _asgame_instance))
    (:`then_3`
      (`GameplayStatics.OpenLevel` "retroAestheticHons"))
    (:`then_4`
      (if (not (< (`self.BR74KillCount`) 5))
        (set `/Game/BluePrint/gameInstance.InsBR74KillCount` (`self.BR74KillCount`) _asgame_instance)))))

(event `UpdateTransform`
  ;[1 1 1] Current Transform
  (set `self.lasttransform` (`self.GetTransform`)))

(event `InputAxis|Move`
  (params (AxisValue :type "Float (single-precision)"))
  ;[1 1 1] Movement
  (`/Engine/EditorBlueprintResources/StandardMacros.CompareFloat` AxisValue
    (:`>`
      (set `self.bisMovingRight` true))
    (:`<`
      (set `self.bisMovingRight` false)))
  (`self.AddMovementInput` (0.25 0.0 0.0) AxisValue))

(event `EnergyRotXYZEvent`
  ;[1 1 1] Spawn Location Fix For Energy Actions
  (if (`self.bisMovingRight`)
    (set `self.energyrotX` 65.0)
    (set `self.energyrotY` 0.1)
    (else
      (set `self.energyrotX` -65.0)
      (set `self.energyrotY` 0.1))))

(event `InputAction|Jump`
  (params (Key :type "Key Structure"))
  ;[1 1 1] Jumping Animation and controller
  (:`Pressed`
    (`self.Jump`)
    (if (`self.CanJump`)
      (`self.Set FlipBook` "NewEnumerator2")
      (`KismetSystemLibrary.Delay` 0.01)
      (if (`NavMovementComponent.IsFalling` (`self.CharacterMovement`))
        (`self.Set FlipBook` "NewEnumerator0"))))
  (:`Released`
    (`self.StopJumping`)))

(event `self.OnLanded`
  (params (Hit :type "HitResult Structure (by ref)"))
  ;[1 1 1] event on land
  (set `self.bJustLanded` Hit_bBlockingHit))

(event `Health_z15`
  (params (healthadded :type Integer))
  ;[1 1 1] heal z15
  (bind _output_get (set `self.Z15_Health` (+ (`self.Z15_Health`) healthadded)))
  (if (>= _output_get 100)
    (set `self.Z15_Health` 100)
    (else
      (`KismetSystemLibrary.PrintString` (`KismetStringLibrary.Conv_IntToString` (`self.Z15_Health`)) true true (struct :`R` 1.0 :`B` 0.391966 :`A` 1.0)))))

(event `Animation Update`
  ;[1 1 1] Idle And Run Controller
  (if (`self.bJustLanded`)
    (`self.Set FlipBook` "NewEnumerator0")
    (`KismetSystemLibrary.Delay` 0.01)
    (set `self.bJustLanded` false)
    (elif (not (`NavMovementComponent.IsFalling` (`self.CharacterMovement`)))
      (`self.Set FlipBook` (select `bool` (> (`KismetMathLibrary.VSize` (`self.GetVelocity`)) 0.0) :`false` "NewEnumerator0" :`true` "NewEnumerator2" :!type "/Game/BluePrint/z15State Enum")))))

(event `InputAction|Energy Shield`
  (params (Key :type "Key Structure"))
  (bind _returnvalue (`SceneComponent.K2_GetComponentToWorld` (`self.CapsuleComponent`)))
  ;[1 1 1] Energy Shield Spawn
  (:`Pressed`
    (if (`/Game/BluePrint/z15shield.isShieldSpawned` (`self.z15shield`))
      _
      (elif (>= (`self.Energy`) 20)
        (`|SpawnActorFromClass` "/Game/BluePrint/z15shield.z15shield_C" (`KismetMathLibrary.MakeTransform` (`KismetMathLibrary.MakeVector` (.x (.location _returnvalue)) (+ (.y (.location _returnvalue)) (`self.energyrotY`)) (.z (.location _returnvalue))) (.rotation _returnvalue) (.scale _returnvalue)) "Undefined" "OverrideRootScale" null null)
        (set `self.Energy` (- (`self.Energy`) 20))))))

(event `Set Spawn`
  ;[1 1 1] Set Spawn Location
  (switch `int` (`self.lvlcounter`)
    (:`Default`
      (set `self.Spawn Loc` (173.0 0.0 -358.0)))
    (:`0`
      (set `self.Spawn Loc` (173.0 0.0 -350.0)))
    (:`1`
      (set `self.Spawn Loc` (136.0 0.0 -1054.0)))
    (:`2`
      (set `self.Spawn Loc` (2024.0 0.0 -970.0)))))

(event `health to float`
  ;[1 1 1] health to float
  (set `self.healthfloat` (/ (`KismetMathLibrary.Conv_IntToDouble` (`self.Z15_Health`)) 100.0)))

(event `Direction`
  (bind _returnvalue_x (`KismetMathLibrary.BreakVector` (`self.GetVelocity`)))
  (bind _returnvalue (`self.GetController`))
  ;[1 1 1] DirectionFlip
  (`/Engine/EditorBlueprintResources/StandardMacros.CompareFloat` _returnvalue_x
    (:`>`
      (`Controller.SetControlRotation` _returnvalue (`KismetMathLibrary.MakeRotator` 0.0) :!label _label))
    (:`==`
      (if (`self.bisMovingRight`)
        (goto _label)
        (else
          (`Controller.SetControlRotation` _returnvalue (`KismetMathLibrary.MakeRotator` 0.0 0.0 180.0) :!label _label_2))))
    (:`<`
      (goto _label_2))))

(event `DMG_Z15`
  (params (NewParamDMGTaken :type Integer))
  ;[1 1 1] damage z15
  (`/Engine/EditorBlueprintResources/StandardMacros.DoOnce` false :!label _label_3
    (:`Completed`
      (bind _output_get (set `self.Z15_Health` (- (`self.Z15_Health`) NewParamDMGTaken)))
      (if (<= _output_get 0)
        (`self.IfDestroyed`)
        (else
          (`KismetSystemLibrary.PrintString` (`KismetStringLibrary.Conv_IntToString` (`self.Z15_Health`)) true true (struct :`R` 1.0 :`B` 0.059606 :`A` 1.0))
          (goto _label_3 :!via `Reset`))))))

(event `energy to float`
  ;[1 1 1] energy to float
  (set `self.Energyfloat` (/ (`KismetMathLibrary.Conv_IntToDouble` (`self.Energy`)) 100.0)))

(event `InputAction|Energy Shoot`
  (params (Key :type "Key Structure"))
  (bind _returnvalue (`SceneComponent.K2_GetComponentToWorld` (`self.arrowshot`)))
  ;[1 1 1] Energy Shoot
  (:`Pressed`
    (if (`NavMovementComponent.IsFalling` (`self.CharacterMovement`))
      _
      (elif (>= (`self.Energy`) 50)
        (`self.DisableInput` null)
        (set `self.Energy` (- (`self.Energy`) 50))
        (`|SpawnActorFromClass` "/Game/BluePrint/energybullet.energybullet_C" (`KismetMathLibrary.MakeTransform` (`KismetMathLibrary.MakeVector` (+ (.x (.location _returnvalue)) (`self.energyrotX`)) (.y (.location _returnvalue)) (.z (.location _returnvalue))) (.rotation _returnvalue) (2.0 2.0 2.5)) "Undefined" "OverrideRootScale" null null)
        (`KismetSystemLibrary.Delay` 1.5)
        (`self.EnableInput` null)))))

(event `self.ReceiveTick`
  (params (DeltaSeconds :type "Float (single-precision)"))
  ;[1 1 1] Event Tick Shoot + Custom Events
  (`|ExecutionSequence`
    (:`then_0`
      (`self.Direction`)
      (`self.Animation Update`)
      (`self.health to float`)
      (`self.energy to float`)
      (`self.EnergyRotXYZEvent`)
      (`self.UpdateTransform`))
    (:`then_1`
      (`/Engine/EditorBlueprintResources/StandardMacros.Gate` true :!label _label_4
        (:`Exit`
          (`/Engine/EditorBlueprintResources/StandardMacros.DoOnce` false :!label _label_5
            (:`Completed`
              (`|SpawnActorFromClass` "/Game/BluePrint/bullet.bullet_C" (`SceneComponent.K2_GetComponentToWorld` (`self.arrowshot`)) "Undefined" "OverrideRootScale" null null)
              (`GameplayStatics.PlaySoundAtLocation` "/Game/Audio/lazer1_Cue.lazer1_Cue")
              (`KismetSystemLibrary.Delay` (`self.shootDelay`))
              (goto _label_5 :!via `Reset`))))))))

(event `InputAction|Shoot`
  (params (Key :type "Key Structure"))
  ;[1 1 1] Event Tick Shoot + Custom Events
  (:`Pressed`
    (goto _label_4 :!via `Open`))
  (:`Released`
    (goto _label_4 :!via `Close`)))

(event `self.CapsuleComponent.OnComponentBeginOverlap`
  (params (OverlappedComponent :type "PrimitiveComponent Object Reference") (OtherActor :type "Actor Object Reference") (OtherComp :type "PrimitiveComponent Object Reference") (OtherBodyIndex :type Integer) (bFromSweep :type Boolean) (SweepResult :type "HitResult Structure (by ref)"))
  ;[1 1 1] Lvl End New Location
  (`|ExecutionSequence`
    (:`then_0`
      (cast `/Game/BluePrint/lvl1End` OtherActor)
      (if (not (< (`self.BR74KillCount`) 5))
        (`self.DisableInput` null)
        (`/Engine/EditorBlueprintResources/StandardMacros.DoOnce` false
          (:`Completed`
            (set `self.lvlcounter` (+ 1 (`self.lvlcounter`)))
            (`self.Set Spawn`)
            (`SceneComponent.K2_SetWorldLocation` (`self.CapsuleComponent`) (`self.Spawn Loc`) false false)
            (`self.Set Spawn`)
            (`KismetSystemLibrary.Delay` 1.0)
            (`self.EnableInput` null)))))
    (:`then_1`
      (cast `/Game/BluePrint/lvl2End1` OtherActor)
      (if (not (< (`self.BR74KillCount`) 7))
        (`self.DisableInput` null)
        (`/Engine/EditorBlueprintResources/StandardMacros.DoOnce` false
          (:`Completed`
            (set `self.lvlcounter` (+ 1 (`self.lvlcounter`)))
            (`self.Set Spawn`)
            (`SceneComponent.K2_SetWorldLocation` (`self.CapsuleComponent`) (`self.Spawn Loc`) false false)
            (`self.Set Spawn`)
            (`KismetSystemLibrary.Delay` 1.0)
            (`self.EnableInput` null)))))))

(fn `Set FlipBook`
  (params (nextstate :type "/Game/BluePrint/z15State Enum" :default "NewEnumerator0"))
  (set `self.CurrentState` nextstate)
  (`PaperFlipbookComponent.SetFlipbook` (`self.Sprite`) (select `/Game/BluePrint/z15State` (`self.CurrentState`) :`NewEnumerator0` (`self.FB_Idle`) :`NewEnumerator2` (`self.FB_moveRight`)))
  (return))

(fn `UserConstructionScript`)