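; BR74_Bullet is a Paper2D projectile that damages Z15 or is blocked by its shield, and self-destructs after a short lifetime.
; Box overlap zeroes damage while the shield is spawned, then stops movement, disables collision and plays a boom sound.
; StateSwitch swaps the flipbook from Idle to Boom before destruction.
; YForward, run every tick, pins the sprite slightly off the Y plane according to its yaw.
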(event `self.ReceiveBeginPlay`
  (`KismetSystemLibrary.Delay` 1.5)
  (`self.K2_DestroyActor`))

(event `YForward`
  (bind (_returnvalue_x _returnvalue_y _returnvalue_z) (`KismetMathLibrary.BreakVector` (`SceneComponent.K2_GetComponentLocation` (`self.PaperFlipbook`))))
  (bind (_returnvalue_roll _returnvalue_pitch _returnvalue_yaw) (`KismetMathLibrary.BreakRotator` (`SceneComponent.K2_GetComponentRotation` (`self.PaperFlipbook`))))
  (bind (_returnvalue_x_2 _returnvalue_y_2 _returnvalue_z_2) (`KismetMathLibrary.BreakVector` (`SceneComponent.K2_GetComponentLocation` (`self.PaperFlipbook`))))
  (if (== _returnvalue_yaw 180.0)
    (`SceneComponent.K2_SetWorldLocation` (`self.PaperFlipbook`) (`KismetMathLibrary.MakeVector` _returnvalue_x -0.1 _returnvalue_z) false false)
    (else
      (`SceneComponent.K2_SetWorldLocation` (`self.PaperFlipbook`) (`KismetMathLibrary.MakeVector` _returnvalue_x_2 0.1 _returnvalue_z_2) false false))))

(event `self.ReceiveTick`
  (params (DeltaSeconds :type "Float (single-precision)"))
  (`self.YForward`))

(event `self.Box.OnComponentBeginOverlap`
  (params (OverlappedComponent :type "PrimitiveComponent Object Reference") (OtherActor :type "Actor Object Reference") (OtherComp :type "PrimitiveComponent Object Reference") (OtherBodyIndex :type Integer) (bFromSweep :type Boolean) (SweepResult :type "HitResult Structure (by ref)"))
  (`|ExecutionSequence`
    (:`then_0`
      (`self.damage0Shield`)
      (`self.YForward`)
      (bind _asz15 (cast `/Game/BluePrint/Z15` OtherActor))
      (`|ExecutionSequence`
        (:`then_0`
          (`MovementComponent.StopMovementImmediately` (`self.ProjectileMovement`)))
        (:`then_1`
          (`/Game/BluePrint/Z15.DMG_Z15` _asz15 (`self.damage`))
          (`PrimitiveComponent.SetCollisionEnabled` (`self.Box`) "NoCollision")
          (`self.State Switch` "NewEnumerator0")
          (`KismetSystemLibrary.Delay` 0.3)
          (`self.K2_DestroyActor`))
        (:`then_2`
          (`GameplayStatics.PlaySoundAtLocation` "/Game/Audio/boom_Cue.boom_Cue"))))
    (:`then_1`
      (`self.YForward`)
      (cast `/Game/BluePrint/z15shield` OtherActor)
      (`PrimitiveComponent.SetCollisionEnabled` (`self.Box`) "NoCollision")
      (`/Engine/EditorBlueprintResources/StandardMacros.DoOnce` false
        (:`Completed`
          (`MovementComponent.StopMovementImmediately` (`self.ProjectileMovement`))
          (`GameplayStatics.PlaySoundAtLocation` "/Game/Audio/boom_Cue.boom_Cue")
          (`self.State Switch` "NewEnumerator0")
          (`KismetSystemLibrary.Delay` 0.3)
          (`self.K2_DestroyActor`))))))

(event `damage0Shield`
  (if (`/Game/BluePrint/z15shield.isShieldSpawned` (`self.z15Shield`))
    (set `self.damage` 0)
    (else
      (set `self.damage` 25))))

(fn `State Switch`
  (params (nextstate :type "/Game/BluePrint/bulletstate Enum" :default "NewEnumerator0"))
  (set `self.currentstate` nextstate)
  (`PaperFlipbookComponent.SetFlipbook` (`self.PaperFlipbook`) (select `/Game/BluePrint/bulletstate` (`self.currentstate`) :`NewEnumerator0` (`self.boom`) :`NewEnumerator1` (`self.Idle`)))
  (return))

(fn `UserConstructionScript`)